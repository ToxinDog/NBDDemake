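; BP_PointManager tracks the BP_PointLight actors near the player and gives them indices by distance, apparently for a four-light limit.
; It attaches to the player pawn; sphere overlaps add or remove lights, and a BeginPlay radius check catches those already inside.
; Each tick a single adjacent-swap pass orders lights nearest first, then updates each with its index.
; SortByDistance is an alternative sort that goes uncalled here.
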(event `self.ReceiveTick`
  (params (DeltaSeconds :type "Float (single-precision)"))
  (bind _sorted_array (`self.SortArray` (`self.PointLights`)))
  (for (_array_element _array_index) _sorted_array
    (bind _asbp_point_light (cast `/Game/GouraudPhong/Blueprints/BP_PointLight` _array_element))
    (set `/Game/GouraudPhong/Blueprints/BP_PointLight.LightIndex` _array_index _asbp_point_light)
    (`KismetSystemLibrary.PrintString` (`KismetStringLibrary.Concat_StrStr` (`KismetSystemLibrary.GetDisplayName` _array_element) " Index: " (`KismetStringLibrary.Conv_IntToString` _array_index)) false false (`KismetMathLibrary.SelectColor` (struct :`R` 1.0 :`A` 1.0) (struct :`G` 1.0 :`A` 1.0) (> _array_index 3)) 0.0)
    (`/Game/GouraudPhong/Blueprints/BP_PointLight.Update` _asbp_point_light)))

(event `self.Sphere.OnComponentBeginOverlap`
  (params (OverlappedComponent :type "PrimitiveComponent Object Reference") (OtherActor :type "Actor Object Reference") (OtherComp :type "PrimitiveComponent Object Reference") (OtherBodyIndex :type Integer) (bFromSweep :type Boolean) (SweepResult :type "HitResult Structure (by ref)"))
  (bind _asbp_point_light (cast `/Game/GouraudPhong/Blueprints/BP_PointLight` OtherActor))
  (`/Engine/EditorBlueprintResources/StandardMacros.IsValid` _asbp_point_light
    (:`Is Valid`
      (bind _returnvalue (`KismetArrayLibrary.Array_Add` (`self.PointLights`) _asbp_point_light))
      (set `/Game/GouraudPhong/Blueprints/BP_PointLight.LightIndex` _returnvalue _asbp_point_light)
      (`/Game/GouraudPhong/Blueprints/BP_PointLight.Update` _asbp_point_light))))

(event `self.ReceiveBeginPlay`
  (bind (_origin _boxextent _sphereradius) (`KismetSystemLibrary.GetComponentBounds` (`self.Sphere`)))
  (`self.K2_AttachToActor` (`GameplayStatics.GetPlayerPawn` 0) "None" "SnapToTarget" "KeepWorld" "KeepWorld")
  ;[1 1 1] Hack for lights overlapping sphere on game start
  (bind _outactors (`GameplayStatics.GetAllActorsOfClass` "/Game/GouraudPhong/Blueprints/BP_PointLight.BP_PointLight_C"))
  (for _array_element _outactors
    (if (<= (`KismetMathLibrary.VSize` (- (`self.K2_GetActorLocation` _array_element) _origin)) _sphereradius)
      (bind _returnvalue (`KismetArrayLibrary.Array_Add` (`self.PointLights`) _array_element))
      (set `/Game/GouraudPhong/Blueprints/BP_PointLight.LightIndex` _returnvalue _array_element)
      (`/Game/GouraudPhong/Blueprints/BP_PointLight.Update` _array_element))))

(event `self.Sphere.OnComponentEndOverlap`
  (params (OverlappedComponent :type "PrimitiveComponent Object Reference") (OtherActor :type "Actor Object Reference") (OtherComp :type "PrimitiveComponent Object Reference") (OtherBodyIndex :type Integer))
  (bind _asbp_point_light (cast `/Game/GouraudPhong/Blueprints/BP_PointLight` OtherActor))
  (`/Engine/EditorBlueprintResources/StandardMacros.IsValid` _asbp_point_light
    (:`Is Valid`
      (`KismetArrayLibrary.Array_RemoveItem` (`self.PointLights`) _asbp_point_light)
      (`/Game/GouraudPhong/Blueprints/BP_PointLight.DisableLight` _asbp_point_light))))

(fn `Compare Distance`
  (params (LocA :type "Vector Structure") (LocB :type "Vector Structure") (Against :type "Vector Structure") (__WorldContext :type "Object Object Reference"))
  (returns (`A Is Closer` :type Boolean))
  (return (< (`KismetMathLibrary.Vector_Distance` LocA Against) (`KismetMathLibrary.Vector_Distance` LocB Against))))

(fn `SortArray`
  (params (`Array ToSort` :type "Array of Actor Object Reference"))
  (returns (`Sorted Array` :type "Array of Actor Object Reference"))
  (locals (Increment :type Integer) (Index :type Integer) (OtherActor :type "Actor Object Reference") (Array :type "Array of Actor Object Reference (by ref)"))
  (bind _index (`local.Index`))
  (bind _returnvalue (select `bool` (== (`local.Increment`) -1) :`false` (`self.ArrayToSort`) :`true` (`local.Array`)))
  (set `self.ArrayToSort` `Array ToSort`)
  (for (_array_element _array_index) _returnvalue
    (set `local.Index` _array_index)
    (bind _returnvalue_2 (+ _array_index 1))
    (if (`KismetArrayLibrary.Array_IsValidIndex` _returnvalue _returnvalue_2)
      (bind _a_is_closer (`self.Compare Distance` (`self.K2_GetActorLocation` _array_element) (`self.K2_GetActorLocation` (`|GetArrayItem` _returnvalue _returnvalue_2)) (`self.K2_GetActorLocation` (`GameplayStatics.GetPlayerPawn` 0))))
      (if (not _a_is_closer)
        (`KismetArrayLibrary.Array_Swap` (`self.ArrayToSort`) _index (+ _index 1))
        (`/Engine/EditorBlueprintResources/StandardMacros.IncrementInt` (`local.Increment`)))))
  (return (`self.ArrayToSort`)))

(fn `SortByDistance`
  (params (Array :type "Array of Actor Object Reference") (RelativeTo :type "Actor Object Reference"))
  (returns (Output :type "Array of Actor Object Reference"))
  (locals (Distances :type "Array of Float (double-precision)") (`New Indexes` :type "Array of Integer") (Result :type "Array of Actor Object Reference"))
  (bind _distances (`local.Distances`))
  (bind _new_indexes (`local.New Indexes`))
  (bind _result (`local.Result`))
  (bind _indexofminvalue (`KismetMathLibrary.MinOfFloatArray` _distances))
  (for _array_element Array
    (`/Engine/EditorBlueprintResources/StandardMacros.IsValid` _array_element
      (:`Is Valid`
        (`KismetArrayLibrary.Array_Add` _distances (`self.GetDistanceTo` RelativeTo _array_element)))))
  (`/Engine/EditorBlueprintResources/StandardMacros.ReverseForEachLoop` _distances
    (:`LoopBody`
      (`KismetArrayLibrary.Array_Add` _new_indexes _indexofminvalue)
      (`KismetArrayLibrary.Array_Remove` _distances _indexofminvalue))
    (:`Completed`
      (for _array_element_2 _new_indexes
        (`KismetArrayLibrary.Array_Add` _result (`|GetArrayItem` Array _array_element_2)))
      (return _result))))

(fn `UserConstructionScript`
  (`SphereComponent.SetSphereRadius` (`self.Sphere`) (`self.ActiveLightRadius`) true))