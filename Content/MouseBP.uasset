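; MouseBP is a mouse threat actor that attacks Seek after staying in contact for too long.
; Tick checks overlap with both Seek and SeekObject, using paired DoOnce gates to start or cancel growling, a camera fade and a kill timer.
; Kill calls Seek's MouseAttack and destroys the mouse, with a delayed load of level NBD chained after destruction.
; An older sphere end-overlap fade path is left disconnected.
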(event `self.ReceiveTick`
  (params (DeltaSeconds :type "Float (single-precision)"))
  (bind _returnvalue (`GameplayStatics.GetPlayerCameraManager` 0))
  (`|ExecutionSequence`
    (:`then_0`
      (if (`self.IsOverlappingActor` (`self.Seek`))
        (if (`self.IsOverlappingActor` (`self.SeekObject`))
          (set `self.Spotted?` true)
          (`/Engine/EditorBlueprintResources/StandardMacros.DoOnce` false :!label _label
            (:`Completed`
              (`AudioComponent.Play` (`self.Growling_Cue`) 0.0)
              (`PlayerCameraManager.StartCameraFade` :`self` _returnvalue :`FromAlpha` 1.0 :`Duration` 0.3)
              (bind _returnvalue_2 (`KismetSystemLibrary.K2_SetTimerDelegate` (delegate `Kill`) (`self.KillTimer`)))
              (set `self.Timer` _returnvalue_2)
              (goto _label_2 :!via `Reset`)))
          (else
            _)))
      (`/Engine/EditorBlueprintResources/StandardMacros.DoOnce` true :!label _label_2
        (:`Completed`
          (`PlayerCameraManager.StartCameraFade` :`self` _returnvalue :`FromAlpha` 1.0 :`Duration` 0.3)
          (`AudioComponent.Stop` (`self.Growling_Cue`))
          (set `self.Spotted?` false)
          (`KismetSystemLibrary.K2_ClearAndInvalidateTimerHandle` (`self.Timer`))
          (goto _label :!via `Reset`))))))

(event `Kill`
  (`/Engine/EditorBlueprintResources/StandardMacros.DoOnce` false
    (:`Completed`
      (`/Game/FirstPersonBP/Blueprints/FirstPersonCharacter.MouseAttack` (`self.Seek`))
      (`self.K2_DestroyActor`)
      (`KismetSystemLibrary.Delay` 10.0)
      (`GameplayStatics.OpenLevel` "NBD"))))

(event `self.ReceiveBeginPlay`
  (`AudioComponent.Stop` (`self.Growling_Cue`)))

(event `self.Sphere.OnComponentEndOverlap`
  (params (OverlappedComponent :type "PrimitiveComponent Object Reference") (OtherActor :type "Actor Object Reference") (OtherComp :type "PrimitiveComponent Object Reference") (OtherBodyIndex :type Integer)))

(fn `UserConstructionScript`)